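; Lever actor that the player rotates between two end positions to change progress in the Tardis game mode.
; Rotate smoothly aims the pitch at a supplied point within clamped limits; reaching the opposite end flips ActiveState, clears the highlight and adds progress.
; Highlighton enables custom-depth highlighting, calls CheckResult and resets DoOnce gates that govern progress deductions during partial pulls.
; A penalty for pulling an unhighlighted lever is unconnected.
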(event `self.highlightOn`
  ;[1 1 1] reset
  (`PrimitiveComponent.SetRenderCustomDepth` (`self.StaticMesh`) true)
  (set `self.isHighlighted` true)
  (`self.Check result`)
  (`|ExecutionSequence`
    (:`then_0`
      (goto _label :!via `Reset`))
    (:`then_1`
      (goto _label_2 :!via `Reset`))))

(event `/Game/Fifis_staf/BP/Interaction_BPI.Rotate`
  (params (PointLocation :type "Vector Structure"))
  (bind (_returnvalue_roll _returnvalue_pitch) (`KismetMathLibrary.BreakRotator` (`self.K2_GetActorRotation`)))
  (bind (_returnvalue_roll_2 _returnvalue_pitch_2) (`KismetMathLibrary.BreakRotator` (`self.K2_GetActorRotation`)))
  (bind (_returnvalue_roll_3 _returnvalue_pitch_3) (`KismetMathLibrary.BreakRotator` (`KismetMathLibrary.RInterpTo` (`self.K2_GetActorRotation`) (`KismetMathLibrary.FindLookAtRotation` (`self.K2_GetActorLocation`) PointLocation) (`GameplayStatics.GetWorldDeltaSeconds`) 20.0)))
  (`self.K2_SetActorRotation` (`KismetMathLibrary.MakeRotator` 0.0 (`KismetMathLibrary.FClamp` _returnvalue_pitch_3 (`self.target rotation`) 0.0)))
  (if (`self.activeState`)
    (if (== _returnvalue_pitch 0.0)
      (set `self.activeState` false)
      (`self.highlightOff`)
      (`/Game/Fifis_staf/BP/Tardis_GM.Change Progress` (`self.As Tardis GM`) 0.25)
      (else
        (`/Engine/EditorBlueprintResources/StandardMacros.DoOnce` false :!label _label
          (:`Completed`
            (`/Game/Fifis_staf/BP/Tardis_GM.Change Progress` (`self.As Tardis GM`) -0.25)))))
    (elif (== _returnvalue_pitch_2 (`self.target rotation`))
      (set `self.activeState` true)
      (`self.highlightOff`)
      (`/Game/Fifis_staf/BP/Tardis_GM.Change Progress` (`self.As Tardis GM`) 0.25)
      (else
        (`/Engine/EditorBlueprintResources/StandardMacros.DoOnce` false :!label _label_2
          (:`Completed`
            (`/Game/Fifis_staf/BP/Tardis_GM.Change Progress` (`self.As Tardis GM`) -0.25)))))))

(fn `UserConstructionScript`
  (`parent.UserConstructionScript`))