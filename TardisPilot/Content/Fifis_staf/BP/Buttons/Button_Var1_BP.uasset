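; Button variant Blueprint for the Tardis game mode that the player interacts with to raise or lower progress.
; It sets a two-second interact time on BeginPlay; interacting plays a sound and a camera shake at the character, then a timeline moves the mesh along Z.
; When the timeline finishes, it turns off the highlight and adds progress if the button was highlighted, or subtracts a smaller amount otherwise.
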(event `self.ReceiveBeginPlay`
  (`parent.ReceiveBeginPlay`)
  (`self.Set_Time_To_Interact` 2.0))

(event `/Game/Fifis_staf/BP/Interaction_BPI.Interact`
  (bind (_relativelocation_x _relativelocation_y) (`KismetMathLibrary.BreakVector` (`SceneComponent.RelativeLocation` (`self.StaticMesh`))))
  (`GameplayStatics.PlaySound2D` (`self.Cue`) 1.0 1.0 0.0 null null)
  (`GameplayStatics.PlayWorldCameraShake` "/Game/Fifis_staf/BP/CameraShake/ButtonCameraShake_BP.ButtonCameraShake_BP_C" (`self.K2_GetActorLocation` (`/Game/Fifis_staf/BP/Tardis_GM.As Character BP` (`self.As Tardis GM`))) 0.0 500.0)
  (bind (_direction _newtrack_0) (`Timeline|Timeline` :!via `PlayFromStart`)
    (:`Update`
      (`SceneComponent.K2_SetRelativeLocation` (`self.StaticMesh`) (`KismetMathLibrary.MakeVector` _relativelocation_x _relativelocation_y _newtrack_0) false false))
    (:`Finished`
      (if (`self.isHighlighted`)
        (`self.highlightOff`)
        (`/Game/Fifis_staf/BP/Tardis_GM.Change Progress` (`self.As Tardis GM`) 0.1)
        (else
          (`self.highlightOff`)
          (`/Game/Fifis_staf/BP/Tardis_GM.Change Progress` (`self.As Tardis GM`) -0.05))))))

(fn `UserConstructionScript`
  (`parent.UserConstructionScript`))