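; Variant 3 of an interactable button, a child Blueprint whose mesh toggles between two rotations when used.
; On BeginPlay it sets a two-second interact time, caches the mesh's rotation and that of a Target component as end poses, then destroys Target.
; Each Interact plays a 2D sound and a FlipFlop snaps the mesh between those poses.
; Timeline, highlight and game-mode progress logic remains unconnected.
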(event `self.ReceiveBeginPlay`
  (bind _target (`self.target`))
  (`parent.ReceiveBeginPlay`)
  (`self.Set_Time_To_Interact` 2.0)
  (set `self.start` (`SceneComponent.RelativeRotation` (`self.StaticMesh`)))
  (set `self.finish` (`SceneComponent.RelativeRotation` _target))
  (`ActorComponent.K2_DestroyComponent` _target))

(event `/Game/Fifis_staf/BP/Interaction_BPI.Interact`
  (`GameplayStatics.PlaySound2D` (`self.Cue`) 1.0 1.0 0.0 null null)
  (`/Engine/EditorBlueprintResources/StandardMacros.FlipFlop`
    (:`A`
      (`SceneComponent.K2_SetRelativeRotation` (`self.StaticMesh`) (`self.finish`) false false))
    (:`B`
      (`SceneComponent.K2_SetRelativeRotation` (`self.StaticMesh`) (`self.start`) false false))))

(fn `UserConstructionScript`
  (`parent.UserConstructionScript`))