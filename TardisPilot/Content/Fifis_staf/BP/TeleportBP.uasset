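; Two-way teleporter actor: when Active, an actor overlapping either of its two boxes is moved to the other box's location and rotation.
; A shared AbleToTeleport flag is cleared on each jump and restored after TeleportDelay, blocking further teleports during the cooldown.
; The player 0 camera fades out and back in over FadeTime each way, starting after the actor has already moved.
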(event `self.Box1.OnComponentBeginOverlap`
  (params (OverlappedComponent :type "PrimitiveComponent Object Reference") (OtherActor :type "Actor Object Reference") (OtherComp :type "PrimitiveComponent Object Reference") (OtherBodyIndex :type Integer) (bFromSweep :type Boolean) (SweepResult :type "HitResult Structure (by ref)"))
  (bind _box (`self.Box`))
  (if (`self.active`)
    (if (`self.able to teleport`)
      (set `self.able to teleport` false)
      (`self.K2_SetActorLocationAndRotation` OtherActor (`SceneComponent.K2_GetComponentLocation` _box) (`SceneComponent.K2_GetComponentRotation` _box) false false)
      (`self.teleport delay`)
      ;[1 1 1] Comment
      (`PlayerCameraManager.StartCameraFade` :`self` (`GameplayStatics.GetPlayerCameraManager` 0) :`ToAlpha` 1.0 :`Duration` (`self.fade time`))
      (`KismetSystemLibrary.Delay` (`self.fade time`))
      (`PlayerCameraManager.StartCameraFade` :`self` (`GameplayStatics.GetPlayerCameraManager` 0) :`FromAlpha` 1.0 :`Duration` (`self.fade time`)))))

(event `self.Box.OnComponentBeginOverlap`
  (params (OverlappedComponent :type "PrimitiveComponent Object Reference") (OtherActor :type "Actor Object Reference") (OtherComp :type "PrimitiveComponent Object Reference") (OtherBodyIndex :type Integer) (bFromSweep :type Boolean) (SweepResult :type "HitResult Structure (by ref)"))
  (bind _box1 (`self.Box1`))
  (if (`self.active`)
    (if (`self.able to teleport`)
      (set `self.able to teleport` false)
      (`self.K2_SetActorLocationAndRotation` OtherActor (`SceneComponent.K2_GetComponentLocation` _box1) (`SceneComponent.K2_GetComponentRotation` _box1) false false)
      (`self.teleport delay`)
      ;[1 1 1] Comment
      (`PlayerCameraManager.StartCameraFade` :`self` (`GameplayStatics.GetPlayerCameraManager` 0) :`ToAlpha` 1.0 :`Duration` (`self.fade time`))
      (`KismetSystemLibrary.Delay` (`self.fade time`))
      (`PlayerCameraManager.StartCameraFade` :`self` (`GameplayStatics.GetPlayerCameraManager` 0) :`FromAlpha` 1.0 :`Duration` (`self.fade time`)))))

(event `teleport delay`
  (`KismetSystemLibrary.Delay` (`self.teleport_delay`))
  (set `self.able to teleport` true))

(fn `UserConstructionScript`)