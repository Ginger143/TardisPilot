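; StartButton_BP is an interactable, one-shot button that starts the game through Tardis_GM.
; It caches the game mode on BeginPlay, and Interact plays a sound cue before calling its StartGame event.
; StartGame calls the game mode's StartGame and turns off the mesh's custom depth rendering.
; Both events are gated by DoOnce and feed a shared camera shake centred on the game mode's character.
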(event `self.ReceiveBeginPlay`
  (bind _astardis_gm (cast `/Game/Fifis_staf/BP/Tardis_GM` (`GameplayStatics.GetGameMode`)))
  (set `self.Tardis GM` _astardis_gm))

(event `/Game/Fifis_staf/BP/Interaction_BPI.Interact`
  (`/Engine/EditorBlueprintResources/StandardMacros.DoOnce` false
    (:`Completed`
      (`GameplayStatics.PlaySound2D` "/Game/Fifis_staf/Sounds/UI/ButtonCue.ButtonCue" 1.0 1.0 0.0 null null)
      (`self.Start Game`)
      (`GameplayStatics.PlayWorldCameraShake` "/Game/Fifis_staf/BP/ButtonCameraShake_BP.ButtonCameraShake_BP_C" (`self.K2_GetActorLocation` (`/Game/Fifis_staf/BP/Tardis_GM.As Character BP` (`self.Tardis GM`))) 0.0 500.0 :!label _label))))

(event `Start Game`
  (`/Engine/EditorBlueprintResources/StandardMacros.DoOnce` false
    (:`Completed`
      (`/Game/Fifis_staf/BP/Tardis_GM.StartGame` (`self.Tardis GM`))
      (`PrimitiveComponent.SetRenderCustomDepth` (`self.StaticMesh2`) false)
      (goto _label))))

(fn `UserConstructionScript`)