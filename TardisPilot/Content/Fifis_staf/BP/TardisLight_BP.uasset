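; TardisLight_BP is a spotlight Blueprint, named for the TARDIS, that switches between an alert-style blinking look and its normal state.
; ChangeColorandmateral sets the SpotLight to the Color variable and applies the BlinkingLight_M light function material.
; ResetLights restores NormalColor and clears the light function material.
; It has no active Tick or BeginPlay logic, so both events depend on being called.
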(event `self.ReceiveBeginPlay`)

(event `Change Color and materal`
  (bind (_color_b _color_g _color_r _color_a) (break `Color` (`self.color`)))
  (`LightComponent.SetLightColor` (`self.SpotLight`) (`KismetMathLibrary.MakeColor` (`KismetMathLibrary.Conv_ByteToDouble` _color_r) (`KismetMathLibrary.Conv_ByteToDouble` _color_g) (`KismetMathLibrary.Conv_ByteToDouble` _color_b) (`KismetMathLibrary.Conv_ByteToDouble` _color_a)) true)
  (`LightComponent.SetLightFunctionMaterial` (`self.SpotLight`) "/Game/Fifis_staf/Materials/BlinkingLight_M.BlinkingLight_M"))

(event `Reset Lights`
  (bind (_normal_color_b _normal_color_g _normal_color_r _normal_color_a) (break `Color` (`self.normal color`)))
  (`LightComponent.SetLightColor` (`self.SpotLight`) (`KismetMathLibrary.MakeColor` (`KismetMathLibrary.Conv_ByteToDouble` _normal_color_r) (`KismetMathLibrary.Conv_ByteToDouble` _normal_color_g) (`KismetMathLibrary.Conv_ByteToDouble` _normal_color_b) (`KismetMathLibrary.Conv_ByteToDouble` _normal_color_a)) true)
  (`LightComponent.SetLightFunctionMaterial` (`self.SpotLight`) null))

(fn `UserConstructionScript`)