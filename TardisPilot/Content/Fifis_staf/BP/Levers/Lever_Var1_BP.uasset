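; A lever variant for the Tardis game that the player drags between up and down positions to change the game mode's progress.
; Rotate eases the mesh's pitch toward a look-at point, clamped between the two limits, and checks for the end opposite the current ActiveState.
; Reaching it passes a DoOnce gate that adds progress, clears the highlight, flips the state, plays feedback and calls ResetLever.
; The resetlever event re-arms both gates.
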(event `self.ReceiveBeginPlay`
  (`parent.ReceiveBeginPlay`)
  (`self.Set_Time_To_Interact` 3.0))

(event `reset lever`
  (`|ExecutionSequence`
    (:`then_0`
      (goto _label :!via `Reset`))
    (:`then_1`
      (goto _label_2 :!via `Reset`))))

(event `/Game/Fifis_staf/BP/Interaction_BPI.Rotate`
  (params (PointLocation :type "Vector Structure"))
  (bind (_returnvalue_roll _returnvalue_pitch _returnvalue_yaw) (`KismetMathLibrary.BreakRotator` (`SceneComponent.K2_GetComponentRotation` (`self.StaticMesh`))))
  (bind (_relativerotation_roll _relativerotation_pitch) (`KismetMathLibrary.BreakRotator` (`SceneComponent.RelativeRotation` (`self.StaticMesh`))))
  (bind (_relativerotation_roll_2 _relativerotation_pitch_2) (`KismetMathLibrary.BreakRotator` (`SceneComponent.RelativeRotation` (`self.StaticMesh`))))
  (bind (_relativerotation_roll_3 _relativerotation_pitch_3) (`KismetMathLibrary.BreakRotator` (`SceneComponent.RelativeRotation` (`self.StaticMesh`))))
  (bind (_returnvalue_roll_2 _returnvalue_pitch_2) (`KismetMathLibrary.BreakRotator` (`KismetMathLibrary.RInterpTo` (`SceneComponent.K2_GetComponentRotation` (`self.StaticMesh`)) (`KismetMathLibrary.FindLookAtRotation` (`self.K2_GetActorLocation`) PointLocation) (`GameplayStatics.GetWorldDeltaSeconds`) 20.0)))
  (`SceneComponent.K2_SetWorldRotation` (`self.StaticMesh`) (`KismetMathLibrary.MakeRotator` _returnvalue_roll (`KismetMathLibrary.FClamp` _returnvalue_pitch_2 (`self.TargetRotation`) 0.0) _returnvalue_yaw) false false)
  (if (`self.ActiveState`)
    (if (`KismetMathLibrary.NearlyEqual_FloatFloat` _relativerotation_pitch_3 0.0 5.0)
      (`/Engine/EditorBlueprintResources/StandardMacros.DoOnce` true :!label _label
        (:`Completed`
          (`/Game/Fifis_staf/BP/Tardis_GM.Change Progress` (`self.As Tardis GM`) (`self.ProgressGain`))
          (`self.highlightOff`)
          (set `self.ActiveState` false)
          (`GameplayStatics.PlaySound2D` (`self.Cue`) 1.0 1.0 0.0 null null)
          (`self.reset lever`)
          (`GameplayStatics.PlayWorldCameraShake` "/Game/Fifis_staf/BP/CameraShake/LeverCameraShake_BP.LeverCameraShake_BP_C" (`self.K2_GetActorLocation` (`/Game/Fifis_staf/BP/Tardis_GM.As Character BP` (`self.As Tardis GM`))) 0.0 500.0))))
    (elif (or (`KismetMathLibrary.NearlyEqual_FloatFloat` _relativerotation_pitch (`self.TargetRotation`) 5.0) (`KismetMathLibrary.NearlyEqual_FloatFloat` _relativerotation_pitch_2 (+ (`self.TargetRotation`) 360.0) 5.0))
      (`/Engine/EditorBlueprintResources/StandardMacros.DoOnce` false :!label _label_2
        (:`Completed`
          (`/Game/Fifis_staf/BP/Tardis_GM.Change Progress` (`self.As Tardis GM`) (`self.ProgressGain`))
          (`self.highlightOff`)
          (set `self.ActiveState` true)
          (`GameplayStatics.PlaySound2D` (`self.Cue`) 1.0 1.0 0.0 null null)
          (`self.reset lever`)
          (`GameplayStatics.PlayWorldCameraShake` "/Game/Fifis_staf/BP/CameraShake/LeverCameraShake_BP.LeverCameraShake_BP_C" (`self.K2_GetActorLocation` (`/Game/Fifis_staf/BP/Tardis_GM.As Character BP` (`self.As Tardis GM`))) 0.0 500.0))))))

(fn `UserConstructionScript`
  (`parent.UserConstructionScript`))