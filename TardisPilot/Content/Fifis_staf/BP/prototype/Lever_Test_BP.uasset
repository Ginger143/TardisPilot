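; Prototype interactable lever that the player rotates toward a point to add progress to the Tardis game mode.
; Rotate interpolates the mesh pitch toward the point, clamped between upright and a target angle.
; Nearing the end opposite its current state fires a DoOnce that adds progress, clears the highlight, flips the down state and plays a sound.
; ResetLever then re-arms both DoOnce gates for the next throw.
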(event `self.ReceiveBeginPlay`
  (`parent.ReceiveBeginPlay`)
  (`self.Set_Time_To_Interact` 3.0))

(event `reset lever`
  (`|ExecutionSequence`
    (:`then_0`
      (goto _label :!via `Reset`))
    (:`then_1`
      (goto _label_2 :!via `Reset`))))

(event `/Game/Fifis_staf/BP/Interaction_BPI.Rotate`
  (params (PointLocation :type "Vector Structure"))
  (bind (_returnvalue_roll _returnvalue_pitch _returnvalue_yaw) (`KismetMathLibrary.BreakRotator` (`SceneComponent.K2_GetComponentRotation` (`self.StaticMesh`))))
  (bind (_relativerotation_roll _relativerotation_pitch) (`KismetMathLibrary.BreakRotator` (`SceneComponent.RelativeRotation` (`self.StaticMesh`))))
  (bind (_relativerotation_roll_2 _relativerotation_pitch_2) (`KismetMathLibrary.BreakRotator` (`SceneComponent.RelativeRotation` (`self.StaticMesh`))))
  (bind (_relativerotation_roll_3 _relativerotation_pitch_3) (`KismetMathLibrary.BreakRotator` (`SceneComponent.RelativeRotation` (`self.StaticMesh`))))
  (bind (_returnvalue_roll_2 _returnvalue_pitch_2) (`KismetMathLibrary.BreakRotator` (`KismetMathLibrary.RInterpTo` (`SceneComponent.K2_GetComponentRotation` (`self.StaticMesh`)) (`KismetMathLibrary.FindLookAtRotation` (`self.K2_GetActorLocation`) PointLocation) (`GameplayStatics.GetWorldDeltaSeconds`) 20.0)))
  (`SceneComponent.K2_SetWorldRotation` (`self.StaticMesh`) (`KismetMathLibrary.MakeRotator` _returnvalue_roll (`KismetMathLibrary.FClamp` _returnvalue_pitch_2 (`self.TargetRotation`) 0.0) _returnvalue_yaw) false false)
  (if (`self.is currently down `)
    (if (`KismetMathLibrary.NearlyEqual_FloatFloat` _relativerotation_pitch_3 0.0 5.0)
      (`/Engine/EditorBlueprintResources/StandardMacros.DoOnce` true :!label _label
        (:`Completed`
          (`/Game/Fifis_staf/BP/Tardis_GM.Change Progress` (`self.As Tardis GM`) (`self.ProgressGain`))
          (`self.highlightOff`)
          (set `self.is currently down ` false)
          (`GameplayStatics.PlaySound2D` (`self.Cue`) 1.0 1.0 0.0 null null)
          (`self.reset lever`))))
    (elif (or (`KismetMathLibrary.NearlyEqual_FloatFloat` _relativerotation_pitch (`self.TargetRotation`) 5.0) (`KismetMathLibrary.NearlyEqual_FloatFloat` _relativerotation_pitch_2 (+ (`self.TargetRotation`) 360.0) 5.0))
      (`/Engine/EditorBlueprintResources/StandardMacros.DoOnce` false :!label _label_2
        (:`Completed`
          (`/Game/Fifis_staf/BP/Tardis_GM.Change Progress` (`self.As Tardis GM`) (`self.ProgressGain`))
          (`self.highlightOff`)
          (set `self.is currently down ` true)
          (`GameplayStatics.PlaySound2D` (`self.Cue`) 1.0 1.0 0.0 null null)
          (`self.reset lever`))))))

(fn `UserConstructionScript`
  (`parent.UserConstructionScript`))