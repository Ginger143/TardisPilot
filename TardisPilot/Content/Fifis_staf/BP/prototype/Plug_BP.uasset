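; Prototype plug actor that follows a supplied location and briefly turns physical when plugged in.
; Despite its name, the Rotate event only sets the actor's location, and only while ShouldMove is true.
; PlugIn blocks movement, waits, enables physics simulation on the mesh for a short window, then disables it and allows movement again.
; Drop is an empty stub.
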(event `self.ReceiveBeginPlay`
  (`parent.ReceiveBeginPlay`))

(event `/Game/Fifis_staf/BP/Interaction_BPI.Rotate`
  (params (PointLocation :type "Vector Structure"))
  (if (`self.should move`)
    (`self.K2_SetActorLocation` PointLocation)))

(event `/Game/Fifis_staf/BP/Interaction_BPI.Drop`)

(event `PlugIn`
  (bind _staticmesh (`self.StaticMesh`))
  (set `self.should move` false)
  (`KismetSystemLibrary.Delay` 1.0)
  (`PrimitiveComponent.SetSimulatePhysics` _staticmesh true)
  (`KismetSystemLibrary.Delay` 2.0)
  (`PrimitiveComponent.SetSimulatePhysics` _staticmesh false)
  (set `self.should move` true))

(fn `UserConstructionScript`
  (`parent.UserConstructionScript`))