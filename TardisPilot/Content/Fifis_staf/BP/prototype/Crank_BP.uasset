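; Crank_BP is a prototype crank actor whose static mesh turns in yaw through externally callable Rotate and Drop events.
; Each Rotate call interpolates yaw toward half a turn past its current value, giving steady frame-time-scaled spin.
; Drop checks whether the yaw is near a full-turn or zero position and only prints a debug message.
; An unconnected look-at rotation chain remains in the graph, and Tick is disabled.
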(event `/Game/Fifis_staf/BP/Interaction_BPI.Rotate`
  (params (PointLocation :type "Vector Structure"))
  (bind (_relativerotation_roll _relativerotation_pitch _relativerotation_yaw) (`KismetMathLibrary.BreakRotator` (`SceneComponent.RelativeRotation` (`self.StaticMesh`))))
  (`SceneComponent.K2_SetRelativeRotation` (`self.StaticMesh`) (`KismetMathLibrary.MakeRotator` 0.0 0.0 (`KismetMathLibrary.FInterpTo` _relativerotation_yaw (+ _relativerotation_yaw 180.0) (`GameplayStatics.GetWorldDeltaSeconds`) 1.0)) false false))

(event `/Game/Fifis_staf/BP/Interaction_BPI.Drop`
  (bind (_relativerotation_roll _relativerotation_pitch _relativerotation_yaw) (`KismetMathLibrary.BreakRotator` (`SceneComponent.RelativeRotation` (`self.StaticMesh`))))
  (if (or (`KismetMathLibrary.NearlyEqual_FloatFloat` _relativerotation_yaw 0.0 5.0) (`KismetMathLibrary.NearlyEqual_FloatFloat` _relativerotation_yaw 360.0 5.0) (`KismetMathLibrary.NearlyEqual_FloatFloat` _relativerotation_yaw -360.0 5.0))
    (`KismetSystemLibrary.PrintString` "Hello")))

(fn `UserConstructionScript`
  (`parent.UserConstructionScript`))