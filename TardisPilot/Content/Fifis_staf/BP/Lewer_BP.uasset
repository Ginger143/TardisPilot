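; Interactable lever for the Tardis game mode that pivots to follow a supplied point and affects progress.
; Rotate eases mesh pitch toward the point's look-at angle, clamped between TargetRotation and zero.
; Reaching the opposite end flips ActiveState, clears the highlight and adds progress; partial movement deducts progress through DoOnce gates.
; A reset event re-highlights the lever, calls CheckResult and rearms both gates.
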(event `self.ReceiveBeginPlay`
  (`parent.ReceiveBeginPlay`)
  (`self.Set_Time_To_Interact` 3.0))

(event `/Game/Fifis_staf/BP/Interaction_BPI.Rotate`
  (params (PointLocation :type "Vector Structure"))
  (bind (_returnvalue_roll _returnvalue_pitch _returnvalue_yaw) (`KismetMathLibrary.BreakRotator` (`SceneComponent.K2_GetComponentRotation` (`self.StaticMesh`))))
  (bind (_relativerotation_roll _relativerotation_pitch) (`KismetMathLibrary.BreakRotator` (`SceneComponent.RelativeRotation` (`self.StaticMesh`))))
  (bind (_relativerotation_roll_2 _relativerotation_pitch_2) (`KismetMathLibrary.BreakRotator` (`SceneComponent.RelativeRotation` (`self.StaticMesh`))))
  (bind (_returnvalue_roll_2 _returnvalue_pitch_2) (`KismetMathLibrary.BreakRotator` (`KismetMathLibrary.RInterpTo` (`SceneComponent.K2_GetComponentRotation` (`self.StaticMesh`)) (`KismetMathLibrary.FindLookAtRotation` (`self.K2_GetActorLocation`) PointLocation) (`GameplayStatics.GetWorldDeltaSeconds`) 20.0)))
  (`SceneComponent.K2_SetWorldRotation` (`self.StaticMesh`) (`KismetMathLibrary.MakeRotator` _returnvalue_roll (`KismetMathLibrary.FClamp` _returnvalue_pitch_2 (`self.TargetRotation`) 0.0) _returnvalue_yaw) false false)
  (if (`self.activeState`)
    (if (== _relativerotation_pitch_2 0.0)
      (set `self.activeState` false)
      (`self.highlightOff`)
      (`/Game/Fifis_staf/BP/Tardis_GM.Change Progress` (`self.As Tardis GM`) (`self.ProgressGain`))
      (else
        (`/Engine/EditorBlueprintResources/StandardMacros.DoOnce` false :!label _label
          (:`Completed`
            (`/Game/Fifis_staf/BP/Tardis_GM.Change Progress` (`self.As Tardis GM`) (`self.ProgressLoss`))))))
    (elif (== _relativerotation_pitch (`self.TargetRotation`))
      (set `self.activeState` true)
      (`self.highlightOff`)
      (`/Game/Fifis_staf/BP/Tardis_GM.Change Progress` (`self.As Tardis GM`) (`self.ProgressGain`))
      (else
        (`/Engine/EditorBlueprintResources/StandardMacros.DoOnce` false :!label _label_2
          (:`Completed`
            (`/Game/Fifis_staf/BP/Tardis_GM.Change Progress` (`self.As Tardis GM`) (`self.ProgressLoss`))))))))

(event `CustomEvent`
  ;[1 1 1] reset
  (`PrimitiveComponent.SetRenderCustomDepth` (`self.StaticMesh`) true)
  (set `self.isHighlighted` true)
  (`self.Check result`)
  (`|ExecutionSequence`
    (:`then_0`
      (goto _label :!via `Reset`))
    (:`then_1`
      (goto _label_2 :!via `Reset`))))

(fn `UserConstructionScript`
  (`parent.UserConstructionScript`))